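; BP_WorldSpawner scatters plant actors across the world within a box extent when play begins.
; BeginPlay repeatedly calls SpawnNewPlant, which line-traces between random high and low points to find a surface, retrying while NbTry remains.
; A sphere trace at the impact rejects spots near actors implementing Interface_Plants.
; Accepted spots get a PlantActor with random yaw.
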(event EventBeginPlay
  (for _index (range 1 40)
    (CallFunction|SpawnNewPlant)))

(fn ConstructionScript)

(fn SpawnNewPlant
  (bind _box (LocalVariables|GetBox))
  (bind _returnvalue (* _box -1.0))
  (bind _returnvalue_2 (Math|Box|MakeBox (Math|Vector|MakeVector _returnvalue _returnvalue _returnvalue) (Math|Vector|MakeVector _box _box _box)))
  (bind _returnvalue_3 (Class|KismetMathLibrary|RandomPointinBoundingBoxBox _returnvalue_2))
  (bind (_x _y) (Math|Vector|BreakVector _returnvalue_3))
  (LocalVariables|SetFlag false)
  (while (and (not (LocalVariables|GetFlag)) (> (LocalVariables|GetNbTry) 0))
    (Math|Integer|DecrementInt (LocalVariables|GetNbTry)
      (:%20%20
        (bind (_outhit _returnvalue_4) (Collision|LineTraceByChannel (Math|Vector|MakeVector _x _y 1e+04) (Math|Vector|MakeVector _x _y -1e+04) "TraceTypeQuery1" false 0 "None"))
        (if _returnvalue_4
          (bind (_outhits _returnvalue_5) (Collision|MultiSphereTraceByChannel (.ImpactPoint (Collision|BreakHitResult _outhit)) (.ImpactPoint (Collision|BreakHitResult _outhit)) (LocalVariables|GetDistanceCollision) "TraceTypeQuery1" false 0 "None"))
          (if _returnvalue_5
            (bind _array_element (Utilities|Array|ForEachLoopwithBreak _outhits)
              (:LoopBody
                (if (Utilities|DoesObjectImplementInterface (.HitActor (Collision|BreakHitResult _array_element)) "/Game/Interfaces/Interface_Plants.Interface_Plants_C")
                  (LocalVariables|SetPlantDetect true)))
              (:Completed
                (if (LocalVariables|GetPlantDetect)
                  (LocalVariables|SetFlag false)
                  (else
                    (LocalVariables|SetFlag true)
                    (Game|SpawnActorfromClass "/Game/Temporary/PlantActor.PlantActor_C" (Math|Transform|MakeTransform (.ImpactPoint (Collision|BreakHitResult _outhit)) (Math|Rotator|MakeRotator 0.0 0.0 (Math|Random|RandomFloatinRange 0.0 3.6e+02)) "1.000000,1.000000,1.000000") "Undefined" 0 0)))))))))))