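; BP_Plant_Melee is a melee plant enemy Blueprint with an Attack event.
; Attack sphere-traces forward from the actor over Range, with debug drawing enabled.
; On a hit, it sets the CoolDown key on its AIC_Plant controller's blackboard to true, then runs a Delay with nothing after it.
; The hit result applies no damage here, and the construction script only calls the parent's.
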(event EventAttack
  (params (Joueur :type BP%20First%20Person%20Character%20Object%20Reference))
  (bind _returnvalue (Transformation|GetActorLocation))
  (bind _returnvalue_2 (Collision|SphereTraceByChannel _returnvalue (+ _returnvalue (* (Transformation|GetActorForwardVector) (Variables|Default|GetRange))) 2e+01 "TraceTypeQuery3" false 0 "ForDuration"))
  (if _returnvalue_2
    (bind _asaic_plant (Utilities|Casting|CastToAIC_Plant (Pawn|GetController)))
    (AI|Components|Blackboard|SetValueasBool (AI|GetBlackboard _asaic_plant) (Utilities|Name|MakeLiteralName "CoolDown") true)
    (Utilities|FlowControl|Delay (Variables|Default|GetDelay))))

(fn ConstructionScript
  (|CallParentFunction))